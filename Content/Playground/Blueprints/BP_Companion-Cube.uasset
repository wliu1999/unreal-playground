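; BP_Companion-Cube is a companion cube Blueprint that tracks its own health and can spawn a baby leash.
; Health is set at BeginPlay, and the TakeDamage and Heal events adjust it without clamping, printing each new value.
; SpawnBabyLeash spawns a BP_Baby_Leash at the cube's transform and calls AttachLeash on it.
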(event Custom|Spawn%20Baby%20Leash
  ;[1 1 1] Spawn Baby Leash
  (Development|PrintString "Spawn Baby Leash")
  (bind _returnvalue (Game|SpawnActorfromClass "/Game/Playground/Blueprints/Projectiles/BP_Baby_Leash.BP_Baby_Leash_C" (Transformation|GetActorTransform) "Undefined" "MultiplyWithRoot" 0 0))
  (Default|AttachLeash _returnvalue))

(event Custom|Take%20Damage
  (params (Damage :type Integer))
  ;[1 1 1] Take damage
  (bind _output_get (Variables|Default|SetHealth (- (Variables|Default|GetHealth) Damage)))
  (Development|PrintString (Utilities|String|ToString(Integer) _output_get)))

(event Custom|Heal
  (params (HP :type Integer))
  (bind _output_get (Variables|Default|SetHealth (+ (Variables|Default|GetHealth) HP)))
  (Development|PrintString (Utilities|String|ToString(Integer) _output_get)))

(event EventBeginPlay
  (Variables|Default|SetHealth 100))

(event EventTick
  (params (DeltaSeconds :type Float%20%28single-precision%29)))

(fn ConstructionScript)