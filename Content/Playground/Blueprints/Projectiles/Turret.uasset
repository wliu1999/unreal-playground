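; Turret actor that periodically turns toward a BP_CompanionCube actor and fires a bullet at it.
; A looping two-second timer started on BeginPlay triggers FireBullet.
; Each shot sets the turret's yaw from a look-at rotation between its Cube component and the target, keeping pitch and roll flat.
; It then spawns BP_Bullet at the Arrow component's transform.
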(event Custom|Fire%20Bullet
  ;[1 1 1] When the turret is created, make a 2 second loop for the turret to activate the "fire bullet" event
  ;[1 1 1] Get Location of Player
  (bind _returnvalue (Actor|GetActorOfClass "/Game/Playground/Blueprints/BP_Companion-Cube.BP_Companion-Cube_C"))
  (Transformation|SetActorRotation (Math|Rotator|MakeRotator 0.0 0.0 (.Yaw (Math|Rotator|BreakRotator (Math|Rotator|FindLookatRotation (Transformation|GetWorldLocation (Variables|Default|GetCube)) (Transformation|GetWorldLocation (Variables|/Script/Engine.Actor|GetRootComponent _returnvalue))))))) ; Set the rotation of the turret
  ;[1 1 1] Spawn a bullet
  (Game|SpawnActorfromClass "/Game/Playground/Blueprints/Projectiles/BP_Bullet.BP_Bullet_C" (Transformation|GetWorldTransform (Variables|Default|GetArrow)) "AlwaysSpawn" "MultiplyWithRoot" 0 0))

(event EventBeginPlay
  ;[1 1 1] When the turret is created, make a 2 second loop for the turret to activate the "fire bullet" event
  (Utilities|Time|SetTimerbyEvent (delegate Custom|Fire%20Bullet) 2.0 true))

(fn ConstructionScript)